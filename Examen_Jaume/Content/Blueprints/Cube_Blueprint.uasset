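; Cube hazard actor that kills the third-person character when it touches the Box trigger.
; The overlap sets the Death flag on the character's ThirdPerson_AnimBP, waits a second, calls GameOver on the character, then destroys every ThirdPersonCharacter in the level.
; A PlaySoundAtLocation node at the player's position is left unconnected and never runs.
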(event OnComponentBeginOverlap(Box)
  (params (OverlappedComponent :type Primitive%20Component%20Object%20Reference) (OtherActor :type Actor%20Object%20Reference) (OtherComp :type Primitive%20Component%20Object%20Reference) (OtherBodyIndex :type Integer) (bFromSweep :type Boolean) (SweepResult :type Hit%20Result%20Structure%20%28by%20ref%29))
  (bind _asthird_person_character (Utilities|Casting|CastToThirdPersonCharacter OtherActor))
  (bind _outactors (Actor|GetAllActorsOfClass "/Game/ThirdPersonBP/Blueprints/ThirdPersonCharacter.ThirdPersonCharacter_C"))
  (bind _asthird_person_anim_bp (Utilities|Casting|CastToThirdPerson_AnimBP (Components|SkeletalMesh|GetAnimInstance (Variables|/Script/Engine.Character|GetMesh _asthird_person_character))))
  (Variables|/Game/Mannequin/Animations/ThirdPerson_AnimBP.ThirdPerson_AnimBP_C|SetDeath _asthird_person_anim_bp true)
  (Utilities|FlowControl|Delay 1.0)
  (Default|GameOver _asthird_person_character)
  (Actor|DestroyActor _outactors))

(event EventBeginPlay)

(event Collision|EventActorBeginOverlap
  (params (OtherActor :type Actor%20Object%20Reference)))

(event EventTick
  (params (DeltaSeconds :type Float%20%28single-precision%29)))

(fn ConstructionScript)