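; Sphere Blueprint is a coin pickup that adds one to the player's Coin count on ThirdPersonCharacter.
; Any actor overlap toggles the mesh's visibility and disables collision without destroying the actor, then credits player 0 regardless of what overlapped.
; It plays a collapse or explosion 2D sound at random pitch, chosen by the SoundMoneda boolean, which flips afterward.
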(event EventBeginPlay)

(event Collision|EventActorBeginOverlap
  (params (OtherActor :type Actor%20Object%20Reference))
  (Rendering|ToggleVisibility (Variables|Debug|GetStaticMeshComponent) false)
  (Collision|SetActorEnableCollision false)
  (bind _asthird_person_character (Utilities|Casting|CastToThirdPersonCharacter (Game|GetPlayerCharacter 0)))
  (Variables|/Game/ThirdPersonBP/Blueprints/ThirdPersonCharacter.ThirdPersonCharacter_C|SetCoin _asthird_person_character (+ 1 (Variables|/Game/ThirdPersonBP/Blueprints/ThirdPersonCharacter.ThirdPersonCharacter_C|GetCoin _asthird_person_character)))
  (if (Variables|Default|GetSoundMoneda)
    (Audio|PlaySound2D "/Game/StarterContent/Audio/Collapse01.Collapse01" 1.0 (Math|Random|RandomFloat) 0.0 0 0)
    (else
      (Audio|PlaySound2D "/Game/StarterContent/Audio/Explosion01.Explosion01" 1.0 (Math|Random|RandomFloat) 0.0 0 0)))
  (Variables|Default|SetSoundMoneda (not (Variables|Default|GetSoundMoneda))))

(event EventTick
  (params (DeltaSeconds :type Float%20%28single-precision%29)))

(fn ConstructionScript)