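; Door actor that rises by an Elevation offset when a ThirdPersonCharacter overlaps it and the player's character holds at least one coin.
; BeginPlay caches the closed and raised positions, and the overlap check sets Open and prints a debug message without deducting coins.
; Tick eases the actor toward the matching position by lerping from its current location at DeltaSeconds times Speed.
; Nothing resets Open, so the door stays raised.
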(event EventBeginPlay
  (bind _returnvalue (Transformation|GetActorLocation))
  (Variables|Default|SetInitialPos (Transformation|GetActorLocation))
  (Variables|Default|SetUpPos (Math|Vector|MakeVector (.x _returnvalue) (.y _returnvalue) (+ (.z _returnvalue) (Variables|Default|GetElevation)))))

(event Collision|EventActorBeginOverlap
  (params (OtherActor :type Actor%20Object%20Reference))
  (if (== (Utilities|GetClass OtherActor) "/Game/ThirdPersonBP/Blueprints/ThirdPersonCharacter.ThirdPersonCharacter_C")
    (bind _asthird_person_character (Utilities|Casting|CastToThirdPersonCharacter (Game|GetPlayerCharacter 0)))
    (if (> (Variables|/Game/ThirdPersonBP/Blueprints/ThirdPersonCharacter.ThirdPersonCharacter_C|GetCoin _asthird_person_character) 0)
      (Variables|Default|SetOpen true)
      (Development|PrintString "Hello"))))

(event EventTick
  (params (DeltaSeconds :type Float%20%28single-precision%29))
  (if (Variables|Default|GetOpen)
    (Transformation|SetActorLocation (Math|Vector|Lerp(Vector) (Transformation|GetActorLocation) (Variables|Default|GetUpPos) (* DeltaSeconds (Variables|Default|GetSpeed))) false false)
    (else
      (Transformation|SetActorLocation (Math|Vector|Lerp(Vector) (Transformation|GetActorLocation) (Variables|Default|GetInitialPos) (* DeltaSeconds (Variables|Default|GetSpeed))) false false))))

(fn ConstructionScript)